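; Spawner actor that keeps a capped population of BP_Marble actors by spawning them at random points inside its SpawningBox.
; Tick accumulates time and, once SpawnPeriod elapses, spawns a marble with itself as Root and adds it to Balls while below Amount.
; The timer resets only on a spawn, so at the cap it retries every tick.
; DeleteBall removes a marble from the array, freeing a slot.
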(event `Delete Ball`
  (params (Ball :type "/Game/Blueprints/BP_Marble Object Reference"))
  (`BlueprintSetLibrary.Set_Remove` (`self.Balls`) Ball)
  (`KismetSystemLibrary.PrintString` "Ball Deleted"))

(event `self.ReceiveTick`
  (params (DeltaSeconds :type "Float (single-precision)"))
  (bind _output_get (set `self.ElapsedTime` (+ DeltaSeconds (`self.ElapsedTime`))))
  (if (>= _output_get (`self.spawnPeriod`))
    (`self.SpawnMarble`)))

(fn `SpawnMarble`
  (bind _spawningbox (`self.SpawningBox`))
  (if (< (`BlueprintSetLibrary.Set_Length` (`self.Balls`)) (`self.Amount`))
    (bind _returnvalue (`|SpawnActorFromClass` "/Game/Blueprints/BP_Marble.BP_Marble_C" (`KismetMathLibrary.MakeTransform` (`KismetMathLibrary.RandomPointInBoundingBox` (`SceneComponent.K2_GetComponentLocation` _spawningbox) (`BoxComponent.BoxExtent` _spawningbox))) "AdjustIfPossibleButAlwaysSpawn" "OverrideRootScale" null self null))
    (`BlueprintSetLibrary.Set_Add` (`self.Balls`) _returnvalue)
    (set `self.ElapsedTime` 0.0)))

(fn `UserConstructionScript`)